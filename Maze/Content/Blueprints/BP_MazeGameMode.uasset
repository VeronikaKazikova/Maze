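; Game mode for the maze game that manages the start, win and escape-menu screens.
; On BeginPlay it disables Chaos physics sleep, binds to BP_Table's WinningConditionMet dispatcher, shows a timed start overlay, then creates the win widget.
; Winning reveals that widget with the cursor and UI-only input.
; Helper functions called from BP_Table undo this on reset, while EscapeMenu and Continue events open and close the pause widget.
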(event Custom|GameWon
  ;[1 1 1] Showing WBP_Win Widget
  (CallFunction|ShowWinWidget))

(event Custom|EscapeMenu
  ;[1 1 1] Create Esc Menu
  (bind _returnvalue (UserInterface|CreateWidget "/Game/Blueprints/WBP_EscMenu.WBP_EscMenu_C"))
  (bind _output_get (Variables|Default|SetEscWidget _returnvalue))
  (UserInterface|Viewport|AddtoViewport _output_get 0)
  (Variables|/Script/Engine.PlayerController|SetbShowMouseCursor (Game|GetPlayerController 0) true))

(event Custom|Continue
  (bind _escwidget (Variables|Default|GetEscWidget))
  ;[1 1 1] Remove Esc Menu
  (Utilities|IsValid _escwidget
    (:Is%20Valid
      (Widget|RemovefromParent _escwidget)
      (Variables|/Script/Engine.PlayerController|SetbShowMouseCursor (Game|GetPlayerController 0) false))))

(event EventBeginPlay
  (Development|ExecuteConsoleCommand "p.Chaos.Solver.SleepEnabled 0" 0) ; Command For Physics To Not Stop Simulating
  ;[1 1 1] Binding To WinningConditionMet Dispatcher (From BP_Table)
  (bind _asbp_table (Utilities|Casting|CastToBP_Table (Game|Player|GetPlayerPawn 0)))
  (EventDispatchers|BindEventtoWinningConditionMet _asbp_table (delegate Custom|GameWon))
  ;[1 1 1] Creating and destroying starting UI overlay
  (bind _returnvalue (UserInterface|CreateWidget "/Game/Blueprints/WBP_Start.WBP_Start_C"))
  (bind _output_get (Variables|Default|SetStartScreen _returnvalue))
  (UserInterface|Viewport|AddtoViewport _output_get 0)
  (Utilities|FlowControl|Delay 5.5)
  (Widget|RemovefromParent (Variables|Default|GetStartScreen))
  ;[1 1 1] Creating and Hiding WBP_Win Widget, Which Will Be Shown After Winning
  (bind _returnvalue_2 (UserInterface|CreateWidget "/Game/Blueprints/WBP_Win.WBP_Win_C"))
  (bind _output_get_2 (Variables|Default|SetWinningWidget _returnvalue_2))
  (UserInterface|Viewport|AddtoViewport _output_get_2 0))

(fn ConstructionScript)

(fn ShowWinWidget
  (Widget|SetVisibility (Variables|Default|GetWinningWidget) "Visible")
  ;[1 1 1] Showing Cursor
  (Variables|/Script/Engine.PlayerController|SetbShowMouseCursor (Game|GetPlayerController 0) true)
  ;[1 1 1] Switching to UI Mode
  (Input|SetInputModeUIOnly (Game|GetPlayerController 0) 0 "DoNotLock"))

(fn ResettoGameMode
  (Input|SetInputModeGameOnly (Game|GetPlayerController 0)))

(fn HideWinWidget
  (Widget|SetVisibility (Variables|Default|GetWinningWidget) "Hidden")
  (Variables|/Script/Engine.PlayerController|SetbShowMouseCursor (Game|GetPlayerController 0) false))