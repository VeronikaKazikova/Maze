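; BP_Ball is a physics ball actor that works with the BP_Table player pawn.
; On BeginPlay it stores the mesh's starting location and binds to two BP_Table dispatchers.
; The reset dispatcher returns the ball to that location and zeroes its linear velocity.
; The win-condition dispatcher destroys the ball.
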(event Custom|BallReset
  ;[1 1 1] Reseting Ball To Starter Location And Erasing Its Velocity
  (CallFunction|ResetBallMovementandPosition))

(event Custom|DestroyingBall
  ;[1 1 1] Binding Destroying The Ball Actor to WinConditionMet Dispatcher
  (Actor|DestroyActor))

(event EventBeginPlay
  ;[1 1 1] Remembering Starter Location Of a Ball
  (Variables|Default|SetStartLocation (Transformation|GetWorldLocation (Variables|Debug|GetStaticMeshComponent)))
  ;[1 1 1] Binding to ResetBallTime Dispatcher (in BP_Table)
  (bind _asbp_table (Utilities|Casting|CastToBP_Table (Game|Player|GetPlayerPawn 0)))
  (EventDispatchers|BindEventtoResetBallTime _asbp_table (delegate Custom|BallReset))
  ;[1 1 1] Binding Destroying The Ball Actor to WinConditionMet Dispatcher
  (bind _asbp_table_2 (Utilities|Casting|CastToBP_Table (Game|Player|GetPlayerPawn 0)))
  (EventDispatchers|BindEventtoWinningConditionMet _asbp_table_2 (delegate Custom|DestroyingBall)))

(fn ConstructionScript)

(fn ResetBallMovementandPosition
  (Transformation|SetWorldLocation (Variables|Debug|GetStaticMeshComponent) (Variables|Default|GetStartLocation) false false)
  (Physics|SetPhysicsLinearVelocity (Variables|Debug|GetStaticMeshComponent) "0, 0, 0" false "None"))