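; Tiltable maze table that the player rotates with axis input to roll a spawned BP_Ball toward the finish hole.
; Pitch and roll inputs rotate FloorBase, clamped to a fixed tilt range.
; Fall and fire overlap boxes fire the ResetBallTime dispatcher and restore the saved table rotation.
; The winning box fires WinningConditionMet and binds WBP_Win's ResetEvent to respawn the ball and reset the game; Escape opens the game mode's menu.
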(event OnComponentBeginOverlap(ResetBox)
  (params (OverlappedComponent :type Primitive%20Component%20Object%20Reference) (OtherActor :type Actor%20Object%20Reference) (OtherComp :type Primitive%20Component%20Object%20Reference) (OtherBodyIndex :type Integer) (bFromSweep :type Boolean) (SweepResult :type Hit%20Result%20Structure%20%28by%20ref%29))
  ;[1 1 1] Calling ResetBallTime Dispatcher After Falling From Table
  (Utilities|Casting|CastToBP_Ball OtherActor)
  (Default|CallResetBallTime)
  (CallFunction|ResetTableTransform))

(event OnComponentBeginOverlap(WinningBox)
  (params (OverlappedComponent :type Primitive%20Component%20Object%20Reference) (OtherActor :type Actor%20Object%20Reference) (OtherComp :type Primitive%20Component%20Object%20Reference) (OtherBodyIndex :type Integer) (bFromSweep :type Boolean) (SweepResult :type Hit%20Result%20Structure%20%28by%20ref%29))
  ;[1 1 1] Calling WinningConditionMet Dispatcher After Falling Into Finish Hole
  (Utilities|Casting|CastToBP_Ball OtherActor)
  (Default|CallWinningConditionMet)
  ;[1 1 1] Binding Reseting Ball to ResetEvent Dispatcher (from WBP_Win - after pressing reset button)
  (bind _foundwidgets (Widget|GetAllWidgetsOfClass "/Game/Blueprints/WBP_Win.WBP_Win_C" false))
  (EventDispatchers|BindEventtoResetEvent (Utilities|Array|Get(acopy) _foundwidgets) (delegate Custom|ResetBallAfterWin)))

(event OnComponentBeginOverlap(FireBox1)
  (params (OverlappedComponent :type Primitive%20Component%20Object%20Reference) (OtherActor :type Actor%20Object%20Reference) (OtherComp :type Primitive%20Component%20Object%20Reference) (OtherBodyIndex :type Integer) (bFromSweep :type Boolean) (SweepResult :type Hit%20Result%20Structure%20%28by%20ref%29))
  ;[1 1 1] Calling ResetBallTime Dispatcher After Overlapping With Fire Zones
  (Utilities|Casting|CastToBP_Ball OtherActor)
  (Default|CallResetBallTime)
  (CallFunction|ResetTableTransform))

(event OnComponentBeginOverlap(FireBox2)
  (params (OverlappedComponent :type Primitive%20Component%20Object%20Reference) (OtherActor :type Actor%20Object%20Reference) (OtherComp :type Primitive%20Component%20Object%20Reference) (OtherBodyIndex :type Integer) (bFromSweep :type Boolean) (SweepResult :type Hit%20Result%20Structure%20%28by%20ref%29))
  ;[1 1 1] Calling ResetBallTime Dispatcher After Overlapping With Fire Zones
  (Utilities|Casting|CastToBP_Ball OtherActor)
  (Default|CallResetBallTime)
  (CallFunction|ResetTableTransform))

(event OnComponentBeginOverlap(FireBox3)
  (params (OverlappedComponent :type Primitive%20Component%20Object%20Reference) (OtherActor :type Actor%20Object%20Reference) (OtherComp :type Primitive%20Component%20Object%20Reference) (OtherBodyIndex :type Integer) (bFromSweep :type Boolean) (SweepResult :type Hit%20Result%20Structure%20%28by%20ref%29))
  ;[1 1 1] Calling ResetBallTime Dispatcher After Overlapping With Fire Zones
  (Utilities|Casting|CastToBP_Ball OtherActor)
  (Default|CallResetBallTime)
  (CallFunction|ResetTableTransform))

(event OnComponentBeginOverlap(FireBox4)
  (params (OverlappedComponent :type Primitive%20Component%20Object%20Reference) (OtherActor :type Actor%20Object%20Reference) (OtherComp :type Primitive%20Component%20Object%20Reference) (OtherBodyIndex :type Integer) (bFromSweep :type Boolean) (SweepResult :type Hit%20Result%20Structure%20%28by%20ref%29))
  ;[1 1 1] Calling ResetBallTime Dispatcher After Overlapping With Fire Zones
  (Utilities|Casting|CastToBP_Ball OtherActor)
  (Default|CallResetBallTime)
  (CallFunction|ResetTableTransform))

(event OnComponentBeginOverlap(FireBox5)
  (params (OverlappedComponent :type Primitive%20Component%20Object%20Reference) (OtherActor :type Actor%20Object%20Reference) (OtherComp :type Primitive%20Component%20Object%20Reference) (OtherBodyIndex :type Integer) (bFromSweep :type Boolean) (SweepResult :type Hit%20Result%20Structure%20%28by%20ref%29))
  ;[1 1 1] Calling ResetBallTime Dispatcher After Overlapping With Fire Zones
  (Utilities|Casting|CastToBP_Ball OtherActor)
  (Default|CallResetBallTime)
  (CallFunction|ResetTableTransform))

(event OnComponentBeginOverlap(FireBox6)
  (params (OverlappedComponent :type Primitive%20Component%20Object%20Reference) (OtherActor :type Actor%20Object%20Reference) (OtherComp :type Primitive%20Component%20Object%20Reference) (OtherBodyIndex :type Integer) (bFromSweep :type Boolean) (SweepResult :type Hit%20Result%20Structure%20%28by%20ref%29))
  ;[1 1 1] Calling ResetBallTime Dispatcher After Overlapping With Fire Zones
  (Utilities|Casting|CastToBP_Ball OtherActor)
  (Default|CallResetBallTime)
  (CallFunction|ResetTableTransform))

(event OnComponentBeginOverlap(FireBox7)
  (params (OverlappedComponent :type Primitive%20Component%20Object%20Reference) (OtherActor :type Actor%20Object%20Reference) (OtherComp :type Primitive%20Component%20Object%20Reference) (OtherBodyIndex :type Integer) (bFromSweep :type Boolean) (SweepResult :type Hit%20Result%20Structure%20%28by%20ref%29))
  ;[1 1 1] Calling ResetBallTime Dispatcher After Overlapping With Fire Zones
  (Utilities|Casting|CastToBP_Ball OtherActor)
  (Default|CallResetBallTime)
  (CallFunction|ResetTableTransform))

(event Custom|ResetBallAfterWin
  ;[1 1 1] Binding Reseting Ball to ResetEvent Dispatcher (from WBP_Win - after pressing reset button)
  (CallFunction|ResetWholeGame))

(event EventBeginPlay
  ;[1 1 1] Spawning Ball At Start
  (Utilities|FlowControl|Delay 3.0)
  (CallFunction|SpawnBallatStart)
  ;[1 1 1] Saving Starting Transform Of Table
  (Variables|Default|SetTableStartTransform (Transformation|GetActorTransform)))

(event Input|AxisEvents|InputAxisTiltRight
  (params (AxisValue :type Float%20%28single-precision%29))
  ;[1 1 1] Table Movement
  (CallFunction|AddingPitch AxisValue)
  (CallFunction|ClampYRotation))

(event Input|AxisEvents|InputAxisTiltUp
  (params (AxisValue :type Float%20%28single-precision%29))
  ;[1 1 1] Table Movement
  (CallFunction|AddingRoll AxisValue)
  (CallFunction|ClampXRotation))

(event Input|KeyboardEvents|Escape
  (params (Key :type Key%20Structure :default "None"))
  ;[1 1 1] Pressing Escape
  (:Pressed
    (bind _asbp_maze_game_mode (Utilities|Casting|CastToBP_MazeGameMode (Game|GetGameMode)))
    (Default|EscapeMenu _asbp_maze_game_mode)))

(fn ConstructionScript)

(fn SpawnBallatStart
  (Game|SpawnActorfromClass "/Game/Blueprints/BP_Ball.BP_Ball_C" (Math|Transform|MakeTransform (Variables|Default|GetBallStartLocation) "0, 0, 0" (Variables|Default|GetBallStartScale)) "Undefined" 0 0))

(fn ClampXRotation
  (bind _floorbase (Variables|Default|GetFloorBase))
  (bind _relativerotation (Variables|/Script/Engine.SceneComponent|GetRelativeRotation _floorbase))
  (Transformation|SetRelativeRotation (Variables|Default|GetFloorBase) (Math|Rotator|MakeRotator (Math|Float|Clamp(Float) (.roll _relativerotation) -15.0 15.0) (.pitch _relativerotation) (.yaw _relativerotation)) false false))

(fn ClampYRotation
  (bind _floorbase (Variables|Default|GetFloorBase))
  (bind _returnvalue (Transformation|GetWorldRotation _floorbase))
  (Transformation|SetWorldRotation (Variables|Default|GetFloorBase) (Math|Rotator|MakeRotator (.roll _returnvalue) (Math|Float|Clamp(Float) (.pitch _returnvalue) -15.0 15.0) (.yaw _returnvalue)) false false))

(fn AddingPitch
  (params (InputValue :type Float%20%28double-precision%29))
  (Transformation|AddWorldRotation (Variables|Default|GetFloorBase) (Math|Rotator|MakeRotator 0.0 (* InputValue (Variables|Default|GetTiltRightRate)) 0.0) false false))

(fn AddingRoll
  (params (InputValue :type Float%20%28double-precision%29))
  (Transformation|AddLocalRotation (Variables|Default|GetFloorBase) (Math|Rotator|MakeRotator (* InputValue (Variables|Default|GetTiltUpRate)) 0.0 0.0) false false))

(fn ResetWholeGame
  (CallFunction|SpawnBallatStart)
  ;[1 1 1] Reseting Back To Game Mode and Hiding Win Widget
  (bind _asbp_maze_game_mode (Utilities|Casting|CastToBP_MazeGameMode (Game|GetGameMode)))
  (Default|ResettoGameMode _asbp_maze_game_mode)
  (Default|HideWinWidget _asbp_maze_game_mode)
  ;[1 1 1] Reseting Table Start Transform
  (CallFunction|ResetTableTransform))

(fn ResetTableTransform
  (Transformation|SetWorldRotation (Variables|Default|GetFloorBase) (.rotation (Variables|Default|GetTableStartTransform)) false false))